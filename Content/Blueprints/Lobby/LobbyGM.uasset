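; Lobby game mode that manages connected players, character pawns, map settings and kicks before server-traveling to the match.
; PostLogin registers each controller, passes GameInstance server data to its LobbyPC and spawns a base pawn at a random PlayerStart.
; UpdateTodos rebroadcasts the player list and available characters to every LobbyPC and recomputes the can-start flag.
; Logout updates character availability and refreshes the lobby, while character selection respawns and possesses the chosen class.
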(event `Respawn Jugador`
  (params (playerController :type "PlayerController Object Reference"))
  (bind _returnvalue (`Controller.K2_GetPawn` playerController))
  (bind _puntosspawn (`self.puntosSpawn`))
  ;[1 1 1] Spawnea el jugador del personaje cuando llega al lobby o muere
  (if (`KismetSystemLibrary.IsValid` _returnvalue)
    (`self.K2_DestroyActor` _returnvalue))
  (bind _returnvalue_2 (`|SpawnActorFromClass` "/Game/Blueprints/GamePlayMode/Personajes/PersonajeBase.PersonajeBase_C" (`self.GetTransform` (`|GetArrayItem` _puntosspawn (`KismetMathLibrary.RandomIntegerInRange` 0 (- (`KismetArrayLibrary.Array_Length` _puntosspawn) 1)))) "Undefined" "OverrideRootScale" null null))
  (`Controller.Possess` playerController _returnvalue_2)
  (`/Engine/EditorBlueprintResources/StandardMacros.IsValid` (`GameplayStatics.GetPlayerPawn` 0)
    (:`Is Valid`
      (`self.UpdateTodos`))))

(event `self.K2_PostLogin`
  (params (NewPlayer :type "PlayerController Object Reference"))
  ;[1 1 1] Configuración inicial del Lobby, maneja la configuración del lobby para el jugador y spawnea el personaje escogido
  (`/Engine/EditorBlueprintResources/ActorMacros.Switch Has Authority`
    (:`Authority`
      (`KismetArrayLibrary.Array_Add` (`self.totalPlayerControllers`) NewPlayer)
      (bind _outactors (`GameplayStatics.GetAllActorsOfClass` "/Script/Engine.PlayerStart"))
      (set `self.puntosSpawn` _outactors)
      (bind _aspavilion_game_instance (cast `/Game/Blueprints/Global/PavilionGameInstance` (`GameplayStatics.GetGameInstance`)))
      (set `self.nombreServer` (`/Game/Blueprints/Global/PavilionGameInstance.NombreServer` _aspavilion_game_instance))
      (set `self.maxJugadores` (`/Game/Blueprints/Global/PavilionGameInstance.MaxJugadores` _aspavilion_game_instance))
      (bind _aslobby_pc (cast `/Game/Blueprints/Lobby/LobbyPC` NewPlayer))
      (`/Game/Blueprints/Lobby/LobbyPC.SetupInicial` _aslobby_pc (`/Game/Blueprints/Global/PavilionGameInstance.userGameData` _aspavilion_game_instance))
      (`/Game/Blueprints/Lobby/LobbyPC.SetupMenuLobby` _aslobby_pc (`self.nombreServer`))
      (`/Game/Blueprints/Lobby/LobbyPC.ActualizaOpcionesLobby` _aslobby_pc (`self.nombreMapa`) (`self.tiempoMapa`) null)
      (`self.Respawn Jugador` NewPlayer))))

(event `UpdateTodos`
  (bind _totalplayercontrollers (`self.totalPlayerControllers`))
  ;[1 1 1] Actualiza la info de los Lobbys de los jugadores cuando se conecta alguien
  (bind _output_get (set `self.numeroPlayerControllers` (`KismetArrayLibrary.Array_Length` (`self.totalPlayerControllers`))))
  (if (> _output_get 0)
    (`KismetArrayLibrary.Array_Clear` (`self.jugadoresConectados`))
    (for _array_element _totalplayercontrollers
      (bind _aslobby_pc (cast `/Game/Blueprints/Lobby/LobbyPC` _array_element))
      (`KismetArrayLibrary.Array_Add` (`self.jugadoresConectados`) (`/Game/Blueprints/Lobby/LobbyPC.InfoJugador` _aslobby_pc))
      (`/Game/Blueprints/Lobby/LobbyPC.ActualizaNumeroJugadores` _aslobby_pc (`self.numeroPlayerControllers`) (`self.maxJugadores`)))
    (for _array_element_2 _totalplayercontrollers
      (bind _aslobby_pc_2 (cast `/Game/Blueprints/Lobby/LobbyPC` _array_element_2))
      (`/Game/Blueprints/Lobby/LobbyPC.AniadeInfoPlayer` _aslobby_pc_2 (`self.jugadoresConectados`))
      (`/Game/Blueprints/Lobby/LobbyPC.ActualizarPersonajesDisponibles` _aslobby_pc_2 (`self.personajesDisponibles`))
      (`self.addKickList`))
    (for _array_element_3 (`self.jugadoresConectados`)
      (bind (_nivel _iconosacumulados _skinsacumuladas _experienciaactual _experienciasiguientenivel _banderinesacumulados _nombreusuario _emailusuario _contraseniausuario _iconoperfil _rolpartida _clasepersonaje _estado) (break `/Game/Blueprints/Global/InfoJugador` _array_element_3))
      (if (== _clasepersonaje null)
        (set `self.puedoEmpezar` false :!label _label)
        (`self.noEmpezar`)
        (elif (`KismetTextLibrary.EqualEqual_TextText` _estado (`|FormatText` "Preparando"))
          (goto _label)
          (else
            (set `self.puedoEmpezar` true)))))))

(event `LanzarJuego`
  ;[1 1 1] Lanza el juego con el mapa seleccionado
  (switch `int` (`self.idMapa`)
    (:`0`
      (`WidgetLayoutLibrary.RemoveAllWidgets`)
      (`KismetSystemLibrary.ExecuteConsoleCommand` "servertravel /Game/Maps/Mapa1" (`GameplayStatics.GetPlayerController` 0)))))

(event `serverAcutalizarModoJuego`
  (params (fotoMapa :type "Texture2D Object Reference") (nombreMapa :type Text) (tiempoMapa :type Text) (idMapa :type Integer))
  ;[1 1 1] Server actualiza la info del lobby de todos los jugadores
  (set `self.fotoMapa` fotoMapa)
  (set `self.nombreMapa` nombreMapa)
  (set `self.tiempoMapa` tiempoMapa)
  (set `self.idMapa` idMapa)
  (for _array_element (`self.totalPlayerControllers`)
    (bind _aslobby_pc (cast `/Game/Blueprints/Lobby/LobbyPC` _array_element))
    (`/Game/Blueprints/Lobby/LobbyPC.ActualizaOpcionesLobby` _aslobby_pc nombreMapa tiempoMapa fotoMapa)))

(event `teHanEchado`
  (params (idJugador :type Integer))
  ;[1 1 1] Echa a un jugador del lobby
  (bind _aslobby_pc (cast `/Game/Blueprints/Lobby/LobbyPC` (`|GetArrayItem` (`self.totalPlayerControllers`) idJugador)))
  (`/Game/Blueprints/Lobby/LobbyPC.EchadoDeServer` _aslobby_pc))

(event `self.K2_OnLogout`
  (params (ExitingController :type "Controller Object Reference"))
  (bind _totalplayercontrollers (`self.totalPlayerControllers`))
  ;[1 1 1] Evento para logout // Borra un cliente del lobby
  (for (_array_element _array_index) _totalplayercontrollers
    (if (== _array_element ExitingController)
      (break)))
  (bind _aslobby_pc (cast `/Game/Blueprints/Lobby/LobbyPC` (`|GetArrayItem` _totalplayercontrollers _array_index)))
  (`KismetArrayLibrary.Array_Set` (`self.personajesDisponibles`) (`/Game/Blueprints/Lobby/LobbyPC.personajeSeleccionado` _aslobby_pc))
  (`KismetArrayLibrary.Array_Remove` (`self.totalPlayerControllers`) _array_index)
  (`KismetArrayLibrary.Array_Remove` (`self.jugadoresConectados`) _array_index)
  (`self.UpdateTodos`))

(event `noEmpezar`)

(event `addKickList`
  ;[1 1 1] Introduce a un jugador en la lista para echarlo si se ha conectado con la lista abierta
  (bind _aslobby_pc (cast `/Game/Blueprints/Lobby/LobbyPC` (`GameplayStatics.GetPlayerController` 0)))
  (bind _menulobbywb (`/Game/Blueprints/Lobby/LobbyPC.menuLobbyWB` _aslobby_pc))
  (`/Engine/EditorBlueprintResources/StandardMacros.IsValid` _menulobbywb
    (:`Is Valid`
      (bind _settings (`/Game/Interfaz/Lobby/MenuLobby.settings` _menulobbywb))
      (if (`Widget.IsVisible` _settings)
        (`/Game/Interfaz/Lobby/MenuOpciones.RellenarVentana` _settings)))))

(event `fijarPersonaje`
  (params (PlayerController :type "PlayerController Object Reference") (ClasePersonaje :type "Character Class Reference"))
  (bind _returnvalue (`Controller.K2_GetPawn` PlayerController))
  (bind _puntosspawn (`self.puntosSpawn`))
  ;[1 1 1] Spawn personaje seleccionado
  (`/Engine/EditorBlueprintResources/StandardMacros.IsValid` _returnvalue
    (:`Is Valid`
      (`self.K2_DestroyActor` _returnvalue))
    (:`Is Not Valid`
      _))
  (bind _returnvalue_2 (`|SpawnActorFromClass` ClasePersonaje (`self.GetTransform` (`|GetArrayItem` _puntosspawn (`KismetMathLibrary.RandomIntegerInRange` 0 (- (`KismetArrayLibrary.Array_Length` _puntosspawn) 1)))) "Undefined" "OverrideRootScale" null null))
  (`Controller.Possess` PlayerController _returnvalue_2))

(fn `OnRep_personajesDisponibles`)

(fn `UserConstructionScript`)