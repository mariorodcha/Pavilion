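; Game instance for Pavilion that handles local user profiles, front-end menus and multiplayer sessions.
; Profiles are GameSave slots keyed by username, with login comparing the stored password directly and Alert widgets reporting account errors.
; Events show menu widgets, host a listen-server Lobby behind a loading screen, and join or destroy sessions.
; Network, travel and session failures route to MuestraMensajeError, though it and both error-to-string converters are empty stubs.
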(event `CargarPerfil`
  (params (id :type String) (psswd :type String))
  (`self.loadUserData` id psswd))

(event `CrearPerfil`
  (params (id :type String) (email :type String) (psswd :type String))
  (`self.createSlot` id email psswd))

(event `self.HandleNetworkError`
  (params (FailureType :type "ENetworkFailure Enum" :default "NetDriverAlreadyExists") (bIsServer :type Boolean))
  ;[1 1 1] Trata NetworkError y muestra mensaje de error
  (if (not bIsServer)
    (`self.MuestraMensajeError` (`self.NetErrorToString` FailureType))))

(event `MuestraMenuPrincipal`
  (bind _returnvalue (`GameplayStatics.GetPlayerController` 0))
  ;[1 1 1] Muestra el menú principal y activa el cursor
  (`/Engine/EditorBlueprintResources/StandardMacros.IsValid` (`self.LoginWB`)
    (:`Is Valid`
      _)
    (:`Is Not Valid`
      (bind _returnvalue_2 (`|CreateWidget` "/Game/Interfaz/CrearPartida/MenuPrincipal.MenuPrincipal_C" _returnvalue))
      (set `self.MenuPrincipalWB` _returnvalue_2)))
  (`UserWidget.AddToViewport` (`self.MenuPrincipalWB`) 0)
  (set `PlayerController.bShowMouseCursor` true _returnvalue))

(event `MuestraPantallaDeCarga`
  ;[1 1 1] Muestra la pantalla de carga
  (`/Engine/EditorBlueprintResources/StandardMacros.IsValid` null
    (:`Is Valid`
      _)
    (:`Is Not Valid`
      (bind _returnvalue (`|CreateWidget` "/Game/Interfaz/Lobby/PantallaDeCarga.PantallaDeCarga_C" (`GameplayStatics.GetPlayerController` 0)))
      (set `self.PantallaCargaWB` _returnvalue)))
  (`UserWidget.AddToViewport` (`self.PantallaCargaWB`) 0))

(event `self.HandleTravelError`
  (params (FailureType :type "ETravelFailure Enum" :default "NoLevel"))
  ;[1 1 1] Trata TravelError y muestra mensaje de error
  (`self.MuestraMensajeError` (`self.TravelErrorToString` FailureType)))

(event `MuestraHostMenu`
  ;[1 1 1] Menú de Host Game
  (`/Engine/EditorBlueprintResources/StandardMacros.IsValid` (`self.MenuHostWB`)
    (:`Is Valid`
      _)
    (:`Is Not Valid`
      (bind _returnvalue (`|CreateWidget` "/Game/Interfaz/CrearPartida/MenuHost.MenuHost_C" (`GameplayStatics.GetPlayerController` 0)))
      (set `self.MenuHostWB` _returnvalue)))
  (`UserWidget.AddToViewport` (`self.MenuHostWB`) 0))

(event `LanzarLobby`
  (params (`ActivarLan?` :type Boolean) (NombreServer :type Text))
  ;[1 1 1] Lanza el lobby con los ajustes del host
  (set `self.NombreServer` NombreServer)
  (`self.MuestraPantallaDeCarga`)
  (`CreateSessionCallbackProxy.CreateSession` (`GameplayStatics.GetPlayerController` 0) (`self.MaxJugadores`) `ActivarLan?`
    (:`OnSuccess`
      (`GameplayStatics.OpenLevel` "Lobby" true "listen"))
    (:`OnFailure`
      (`self.MuestraMensajeError` "Error al crear la sesión. Por favor,  inténtelo de nuevo."))))

(event `DestruyeSesion`
  (params (PlayerController :type "PlayerController Object Reference"))
  ;[1 1 1] Destruye la sesion cuando es llamado
  (`DestroySessionCallbackProxy.DestroySession` PlayerController))

(event `MuestraServerMenu`
  ;[1 1 1] Muestra el menú de server. Se crea cada vez que se llama el evento
  (bind _returnvalue (`|CreateWidget` "/Game/Interfaz/CrearPartida/MenuServer.MenuServer_C" (`GameplayStatics.GetPlayerController` 0)))
  (`UserWidget.AddToViewport` _returnvalue 0))

(event `UnirseAServer`
  (params (SesionALaQueUnirse :type "BlueprintSessionResult Structure"))
  ;[1 1 1] Unirse al servidor, se llama desde el menu de server
  (`XRLoadingScreenFunctionLibrary.ShowLoadingScreen`)
  (`JoinSessionCallbackProxy.JoinSession` (`GameplayStatics.GetPlayerController` 0) SesionALaQueUnirse
    (:`OnFailure`
      (`self.MuestraMensajeError` "Error al unirse al servidor. Por favor, inténtelo de nuevo."))))

(event `MuestraMenuOpciones`
  ;[1 1 1] Muestra el menú de opciones
  (`/Engine/EditorBlueprintResources/StandardMacros.IsValid` (`self.MenuOpcionesWB`)
    (:`Is Valid`
      _)
    (:`Is Not Valid`
      (bind _returnvalue (`|CreateWidget` "/Game/Interfaz/Lobby/MenuOpciones.MenuOpciones_C" (`GameplayStatics.GetPlayerController` 0)))
      (set `self.MenuOpcionesWB` _returnvalue)))
  (`UserWidget.AddToViewport` (`self.MenuOpcionesWB`) 0))

(fn `createSlot`
  (params (username :type String) (email :type String) (contrasenia :type String))
  (bind _array (`|MakeArray` 0))
  (bind _returnvalue (`GameplayStatics.DoesSaveGameExist` username))
  (if _returnvalue
    ;[1 1 1] Mensaje error, ya existe cuenta con ese nombre
    (bind _returnvalue_2 (`|CreateWidget` "/Game/Interfaz/General/Alert.Alert_C"))
    (`/Game/Interfaz/General/Alert.setContenido` _returnvalue_2 "Ya existe una cuenta  \ncon ese nombre.")
    (else
      ;[1 1 1] Si no existe, lo crea
      (bind _returnvalue_3 (`GameplayStatics.CreateSaveGameObject` "/Game/Blueprints/Global/GameSave.GameSave_C"))
      (bind _output_get (set `self.Save Game Data` _returnvalue_3))
      (bind _output_get_2 (set `/Game/Blueprints/Global/GameSave.GameData` (make `/Game/Blueprints/Global/InfoJugador` 1 _array _array 0 200 0 username email contrasenia (make `SlateBrush` (240.0 240.0) (struct) (struct :`SpecifiedColor` (struct :`R` 1.0 :`G` 1.0 :`B` 1.0 :`A` 1.0) :`ColorUseRule` "UseColor_Specified") "/Game/Iconos/Perfil/sniffing-dog.sniffing-dog") "NewEnumerator0" null "Preparando") _output_get))
      (`GameplayStatics.SaveGameToSlot` _output_get (`.nombreUsuario_24_0B63BB79400F21373FA7978773C93E1D` (break `/Game/Blueprints/Global/InfoJugador` _output_get_2))))))

(fn `loadUserData`
  (params (id :type String) (passwd :type String))
  ;[1 1 1] Comprueba si hay fichero con datos guardados
  (bind _returnvalue (`GameplayStatics.DoesSaveGameExist` id))
  (if _returnvalue
    ;[1 1 1] Si existe, lo carga
    (bind _returnvalue_2 (`GameplayStatics.LoadGameFromSlot` id))
    (`/Engine/EditorBlueprintResources/StandardMacros.IsValid` _returnvalue_2
      (:`Is Valid`
        (bind _asgame_save (cast `/Game/Blueprints/Global/GameSave` _returnvalue_2))
        (bind (_gamedata_nivel _gamedata_iconosacumulados _gamedata_skinsacumuladas _gamedata_experienciaactual _gamedata_experienciasiguientenivel _gamedata_banderinesacumulados _gamedata_nombreusuario _gamedata_emailusuario _gamedata_contraseniausuario) (break `/Game/Blueprints/Global/InfoJugador` (`/Game/Blueprints/Global/GameSave.GameData` _asgame_save)))
        (if (`KismetStringLibrary.EqualEqual_StrStr` _gamedata_contraseniausuario passwd)
          (set `self.userGameData` (`/Game/Blueprints/Global/GameSave.GameData` _asgame_save))
          (set `self.Save Game Data` _asgame_save)
          (else
            ;[1 1 1] Mensaje de contraseña incorrecta
            (bind _returnvalue_3 (`|CreateWidget` "/Game/Interfaz/General/Alert.Alert_C"))
            (`/Game/Interfaz/General/Alert.setContenido` _returnvalue_3 "La contraseña es incorrecta.")
            (`UserWidget.AddToViewport` _returnvalue_3 0)))))
    (else
      ;[1 1 1] Muestra mensaje de que no existe cuenta con ese id
      (bind _returnvalue_4 (`|CreateWidget` "/Game/Interfaz/General/Alert.Alert_C"))
      (`/Game/Interfaz/General/Alert.setContenido` _returnvalue_4 "No existe ninguna cuenta con \nese nombre de usuario.")
      (`UserWidget.AddToViewport` _returnvalue_4 0))))

(fn `NetErrorToString`
  (params (TipoFallo :type "ENetworkFailure Enum" :default "NetDriverAlreadyExists"))
  (returns (Output :type String))
  (return ""))

(fn `removeSlot`
  (`GameplayStatics.DeleteGameInSlot` ""))

(fn `saveUserData`
  (bind _save_game_data (`self.Save Game Data`))
  (bind (_nivel _iconosacumulados _skinsacumuladas _experienciaactual _experienciasiguientenivel _banderinesacumulados _nombreusuario) (break `/Game/Blueprints/Global/InfoJugador` (`self.userGameData`)))
  (bind _returnvalue (`GameplayStatics.DoesSaveGameExist` _nombreusuario))
  (if _returnvalue
    (set `/Game/Blueprints/Global/GameSave.GameData` (`self.userGameData`) _save_game_data)
    (`GameplayStatics.SaveGameToSlot` _save_game_data _nombreusuario)))

(fn `TravelErrorToString`
  (params (TipoFallo :type "ETravelFailure Enum" :default "NoLevel"))
  (returns (Output :type String))
  (return ""))