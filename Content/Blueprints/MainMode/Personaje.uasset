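; Player character Blueprint for the main mode that can pick up a flag (Bandera) and carry it on its back.
; Capsule overlap with a Bandera stores it, snaps it to the character at an offset and disables its collision.
; Pressing G re-enables the flag's collision and destroys the character.
; The construction script attaches the weapon (Arma) to the mesh's "Arma" socket.
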(event `self.CapsuleComponent.OnComponentBeginOverlap`
  (params (OverlappedComponent :type "PrimitiveComponent Object Reference") (OtherActor :type "Actor Object Reference") (OtherComp :type "PrimitiveComponent Object Reference") (OtherBodyIndex :type Integer) (bFromSweep :type Boolean) (SweepResult :type "HitResult Structure (by ref)"))
  ;[1 1 1] Coger bandera
  (if (== (`GameplayStatics.GetObjectClass` OtherActor) "/Game/Blueprints/MainMode/Bandera.Bandera_C")
    (bind _asbandera (cast `/Game/Blueprints/MainMode/Bandera` OtherActor))
    (bind _output_get (set `self.Bandera` _asbandera))
    (`self.K2_AttachToActor` _output_get self "None" "SnapToTarget" "SnapToTarget" "KeepRelative" true) ; Se añade la bandera como hija del personaje
    (`self.K2_SetActorRelativeLocation` (`self.Bandera`) (-20.0 0.0 100.0) false true) ; Se modifica la posición relativa de la bandera para que quede a la espalda
    (`self.SetActorEnableCollision` (`self.Bandera`) false)))

(event `Key|G`
  (params (Key :type "Key Structure"))
  (:`Pressed`
    (`self.SetActorEnableCollision` (`self.Bandera`) true)
    (`self.K2_DestroyActor`)))

(fn `UserConstructionScript`
  (`parent.UserConstructionScript`)
  (`SceneComponent.K2_AttachToComponent` (`self.Arma`) (`self.Mesh`) "Arma" "SnapToTarget" "KeepRelative" "KeepRelative" true))