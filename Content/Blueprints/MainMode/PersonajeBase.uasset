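; Base character for a team shooter with flag capture, handling HUD creation, firing, reloading, damage and death.
; Automatic fire loops a Gate through a retriggerable delay, line-tracing from the weapon muzzle along an upward-biased camera direction to damage opposing-team characters.
; Releasing fire auto-reloads an empty magazine.
; Overlapping a flag picks it up; Tick detects zero health, and death respawns any carried flag before destroying the actor.
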(event `self.ReceiveBeginPlay`
  (bind _returnvalue (`|CreateWidget` "/Game/Blueprints/Interfaz/HUDPartida.HUDPartida_C"))
  (bind _output_get (set `self.hud` _returnvalue))
  (`UserWidget.AddToViewport` _output_get 0))

(event `self.ReceiveTick`
  (params (DeltaSeconds :type "Float (single-precision)"))
  (if (== (`self.VidaActual`) 0)
    (`self.Muere`)))

(event `ComienzaDisparo`
  (`|ExecutionSequence`
    (:`then_0`
      (goto _label :!via `Open`))
    (:`then_1`
      (`/Engine/EditorBlueprintResources/StandardMacros.Gate` true :!label _label
        (:`Exit`
          (`|ExecutionSequence`
            (:`then_0`
              (`KismetSystemLibrary.RetriggerableDelay` (`self.CadenciaArma`))
              (goto _label))
            (:`then_1`
              (if (<= (`self.MunicionActual`) 0)
                (`KismetSystemLibrary.PrintString` "sin municion" true true (struct :`R` 1.0 :`B` 0.137316 :`A` 1.0))
                (else
                  (bind _asarma (cast `/Game/Blueprints/MainMode/Arma` (`ChildActorComponent.ChildActor` (`self.Arma`))))
                  (bind _returnvalue (`SceneComponent.GetSocketLocation` (`/Game/Blueprints/MainMode/Arma.SkeletalMesh` _asarma) "MuzzleSocket"))
                  (`GameplayStatics.SpawnEmitterAtLocation` "/Game/FPS_Assault_Pack/Particles/Emitters/Rifle/P_Rifle_Muzzleflash.P_Rifle_Muzzleflash" _returnvalue)
                  (bind (_outhit _returnvalue_2) (`KismetSystemLibrary.LineTraceSingle` :`Start` _returnvalue :`End` (+ _returnvalue (* (`KismetMathLibrary.MakeVector` (.x (`SceneComponent.GetForwardVector` (`self.PlayerCamera`))) (.y (`SceneComponent.GetForwardVector` (`self.PlayerCamera`))) (+ (.z (`SceneComponent.GetForwardVector` (`self.PlayerCamera`))) 0.15)) (`self.RangoArma`))) :`TraceChannel` "TraceTypeQuery1" :`DrawDebugType` "ForDuration" :`DrawTime` 2.0))
                  (bind _output_get (set `self.MunicionActual` (- (`self.MunicionActual`) 1)))
                  (if _returnvalue_2
                    (bind (_bblockinghit _binitialoverlap _time _distance _location _impactpoint _normal _impactnormal _physmat _hitactor) (`GameplayStatics.BreakHitResult` _outhit))
                    (if (== (`GameplayStatics.GetObjectClass` _hitactor) "PersonajeBase_C")
                      (bind _aspersonaje_base (cast `/Game/Blueprints/MainMode/PersonajeBase` _hitactor))
                      (if (!= (`/Game/Blueprints/MainMode/PersonajeBase.idEquipo` _aspersonaje_base) (`self.idEquipo`))
                        (`self.RecibeDaño` _aspersonaje_base (`self.DañoArma`))))))))))))))

(event `TerminaDisparo`
  (goto _label :!via `Close`))

(event `FirePress`
  (set `self.Estado` "NewEnumerator0")
  (if (not (`|EnumEquality` (`self.Estado`) "NewEnumerator1"))
    (`self.ComienzaDisparo`)))

(event `FireRelease`
  (set `self.Estado` "NewEnumerator3")
  (`self.TerminaDisparo`)
  (`self.RecargaAutomatica`))

(event `Muere`
  (set `self.Estado` "NewEnumerator2")
  (set `self.PuedeDisparar` false)
  (`PrimitiveComponent.SetCollisionEnabled` (`self.CapsuleComponent`) "NoCollision")
  (if (`self.TieneBandera`)
    (`KismetSystemLibrary.PrintString` "tiene")
    (set `self.TieneBandera` false)
    (`|SpawnActorFromClass` "/Game/Blueprints/MainMode/Bandera.Bandera_C" (`KismetMathLibrary.MakeTransform` (`SceneComponent.K2_GetComponentLocation` (`self.CapsuleComponent`))) "AlwaysSpawn" "OverrideRootScale" null null)
    (else
      (`KismetSystemLibrary.PrintString` "no tiene")))
  (`KismetSystemLibrary.Delay` 2.5)
  (`self.K2_DestroyActor`))

(event `Recarga`
  (if (`self.PuedeDisparar`)
    (if (== (`self.MunicionActual`) (`self.MunicionMaxima`))
      (`KismetSystemLibrary.PrintString` "full ammo")
      (else
        (set `self.Estado` "NewEnumerator1")
        (set `self.MunicionActual` (`self.MunicionMaxima`))
        (`KismetSystemLibrary.Delay` 2.0)
        (set `self.Estado` "NewEnumerator3")))))

(event `RecargaAutomatica`
  (if (== (`self.MunicionActual`) 0)
    (`self.Recarga`)))

(event `self.CapsuleComponent.OnComponentBeginOverlap`
  (params (OverlappedComponent :type "PrimitiveComponent Object Reference") (OtherActor :type "Actor Object Reference") (OtherComp :type "PrimitiveComponent Object Reference") (OtherBodyIndex :type Integer) (bFromSweep :type Boolean) (SweepResult :type "HitResult Structure (by ref)"))
  (if (== (`GameplayStatics.GetObjectClass` OtherActor) "/Game/Blueprints/MainMode/Bandera.Bandera_C")
    (set `self.TieneBandera` true)
    (`self.K2_DestroyActor` OtherActor)))

(fn `RecibeDaño`
  (params (`Daño` :type Integer))
  (bind _output_get (set `self.VidaActual` (`KismetMathLibrary.Clamp` (- (`self.VidaActual`) `Daño`) 0 (`self.VidaMaxima`))))
  (`KismetSystemLibrary.PrintString` (`KismetStringLibrary.Conv_IntToString` _output_get)))

(fn `UserConstructionScript`
  (`SceneComponent.K2_AttachToComponent` (`self.Arma`) (`self.Mesh`) "weapon" "SnapToTarget" "SnapToTarget" "KeepRelative" true)
  (set `self.MunicionActual` (`self.MunicionMaxima`))
  (set `self.VidaActual` (`self.VidaMaxima`)))