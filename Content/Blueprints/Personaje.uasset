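; Personaje is a character Blueprint that picks up a flag (Bandera) by touching it.
; When its capsule begins overlapping a Bandera, it stores the reference and attaches that actor to itself, snapping location and rotation while keeping relative scale.
; It then teleports the flag to a fixed relative offset behind and above the character's origin.
; No drop or release logic is present, and the construction script only calls its parent.
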(event `self.CapsuleComponent.OnComponentBeginOverlap`
  (params (OverlappedComponent :type "PrimitiveComponent Object Reference") (OtherActor :type "Actor Object Reference") (OtherComp :type "PrimitiveComponent Object Reference") (OtherBodyIndex :type Integer) (bFromSweep :type Boolean) (SweepResult :type "HitResult Structure (by ref)"))
  (if (== (`GameplayStatics.GetObjectClass` OtherActor) "/Game/Blueprints/Bandera.Bandera_C")
    (bind _asbandera (cast `/Game/Blueprints/Bandera` OtherActor))
    (set `self.Bandera` _asbandera)
    (`self.K2_AttachToActor` OtherActor self "None" "SnapToTarget" "SnapToTarget" "KeepRelative" true)
    (`self.K2_SetActorRelativeLocation` (`self.Bandera`) (-20.0 0.0 100.0) false true)))

(fn `UserConstructionScript`
  (`parent.UserConstructionScript`))