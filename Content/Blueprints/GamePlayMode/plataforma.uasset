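; Moving platform Blueprint that shuttles its Cube back and forth along the relative X axis until its lifetime runs out.
; The custom event moverPlataforma stores the starting location, then loops MoveComponentTo out by Distancia and back, each leg taking TiempoMovimiento.
; After each leg it accumulates elapsed time and destroys the actor only when that total exactly equals TiempoMax.
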(event `moverPlataforma`
  (bind _cube (`self.Cube`))
  (bind _cube_2 (`self.Cube`))
  (set `self.locationInicial` (`SceneComponent.RelativeLocation` (`self.Cube`)))
  (`KismetSystemLibrary.MoveComponentTo` _cube (`KismetMathLibrary.MakeVector` (+ (.x (`self.locationInicial`)) (`self.distancia`)) (.y (`self.locationInicial`)) (.z (`self.locationInicial`))) (`SceneComponent.RelativeRotation` _cube) false false (`self.tiempoMovimiento`) :!label _label)
  (set `self.tiempoActual` (+ (`self.tiempoActual`) (`self.tiempoMovimiento`)))
  (if (== (`self.tiempoActual`) (`self.tiempoMax`))
    (`self.K2_DestroyActor`)
    (else
      (`KismetSystemLibrary.MoveComponentTo` _cube_2 (`self.locationInicial`) (`SceneComponent.RelativeRotation` _cube_2) false false (`self.tiempoMovimiento`))
      (set `self.tiempoActual` (+ (`self.tiempoActual`) (`self.tiempoMovimiento`)))
      (if (== (`self.tiempoActual`) (`self.tiempoMax`))
        (`self.K2_DestroyActor`)
        (else
          (goto _label))))))

(fn `UserConstructionScript`)