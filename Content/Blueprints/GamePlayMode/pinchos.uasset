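; Spike hazard (pinchos) that repeatedly damages the player's possessed character while it stands inside the Box trigger.
; Begin overlap accepts only the GamePlayPC's possessed PersonajeBase, via its Mesh component, then stores it and starts the damage loop.
; The loop applies DañoBase through RecibeDaño, waits RatioDaño with a Delay, and repeats until that mesh's end overlap clears the Encima flag.
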(event `aplicarDaño`
  (if (`self.encima`) :!label _label
    (`/Game/Blueprints/GamePlayMode/Personajes/PersonajeBase.RecibeDaño` (`self.pawnEncima`) (`self.dañoBase`))
    (`KismetSystemLibrary.Delay` (`KismetMathLibrary.Conv_IntToDouble` (`self.ratioDaño`)))
    (goto _label)))

(event `self.Box.OnComponentBeginOverlap`
  (params (OverlappedComponent :type "PrimitiveComponent Object Reference") (OtherActor :type "Actor Object Reference") (OtherComp :type "PrimitiveComponent Object Reference") (OtherBodyIndex :type Integer) (bFromSweep :type Boolean) (SweepResult :type "HitResult Structure (by ref)"))
  (bind _asgame_play_pc (cast `/Game/Blueprints/GamePlayMode/GamePlayPC` (`GameplayStatics.GetPlayerController` 0)))
  (bind _pawnposeido (`/Game/Blueprints/GamePlayMode/GamePlayPC.pawnPoseido` _asgame_play_pc))
  (if (== _pawnposeido OtherActor)
    (bind _aspersonaje_base (cast `/Game/Blueprints/GamePlayMode/Personajes/PersonajeBase` _pawnposeido))
    (if (== OtherComp (`Character.Mesh` _aspersonaje_base))
      (set `self.pawnEncima` _aspersonaje_base)
      (set `self.encima` true)
      (`self.aplicarDaño`))))

(event `self.Box.OnComponentEndOverlap`
  (params (OverlappedComponent :type "PrimitiveComponent Object Reference") (OtherActor :type "Actor Object Reference") (OtherComp :type "PrimitiveComponent Object Reference") (OtherBodyIndex :type Integer))
  (if (== (`self.pawnEncima`) OtherActor)
    (if (== OtherComp (`Character.Mesh` (`self.pawnEncima`)))
      (set `self.encima` false))))

(fn `UserConstructionScript`)