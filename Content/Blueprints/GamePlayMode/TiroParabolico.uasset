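; TiroParabolico is a gameplay Blueprint that launches a grenade in a parabolic arc from a character's weapon.
; Its event spawns the given class, scaled down, at the weapon's MuzzleSocket with the player camera's rotation.
; If the spawned actor is a Granada, it sets the mesh's physics velocity along the camera's forward direction, pitched upward at a fixed speed, leaving the arc to physics.
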(event `TiroParabolico`
  (params (clase :type "Actor Class Reference") (personaje :type "/Game/Blueprints/GamePlayMode/Personajes/PersonajeBase Object Reference"))
  (bind _returnvalue (`SceneComponent.K2_GetComponentRotation` (`/Game/Blueprints/GamePlayMode/Personajes/PersonajeBase.PlayerCamera` personaje)))
  (bind _asarma (cast `/Game/Blueprints/GamePlayMode/Arma` (`ChildActorComponent.ChildActor` (`/Game/Blueprints/GamePlayMode/Personajes/PersonajeBase.Arma` personaje))))
  (bind _returnvalue_2 (`|SpawnActorFromClass` clase (`KismetMathLibrary.MakeTransform` (`SceneComponent.GetSocketLocation` (`/Game/Blueprints/GamePlayMode/Arma.SkeletalMesh` _asarma) "MuzzleSocket") _returnvalue (0.1 0.1 0.1)) "Undefined" "OverrideRootScale" null null))
  (bind _asgranada (cast `/Game/Blueprints/GamePlayMode/Granada` _returnvalue_2))
  (`PrimitiveComponent.SetPhysicsLinearVelocity` (`/Game/Blueprints/GamePlayMode/Granada.StaticMesh` _asgranada) (* (`KismetMathLibrary.GetForwardVector` (`KismetMathLibrary.MakeRotator` (.roll _returnvalue) (+ (.pitch _returnvalue) 20.0) (.yaw _returnvalue))) 1500.0) false "None"))