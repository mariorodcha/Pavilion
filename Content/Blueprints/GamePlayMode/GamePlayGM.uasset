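; GamePlayGM is a game mode that gives each joining player a character.
; On HandleStartingNewPlayer it spawns a PersonajeBase at the first Location entry, adjusting for collisions but always spawning, then has that player's controller possess it.
; Logic to start the match once two players are present exists but is disconnected and never runs; Tick and the construction script are empty.
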(event `self.HandleStartingNewPlayer`
  (params (NewPlayer :type "PlayerController Object Reference"))
  (bind _returnvalue (`|SpawnActorFromClass` "/Game/Blueprints/GamePlayMode/Personajes/PersonajeBase.PersonajeBase_C" (`KismetMathLibrary.MakeTransform` (`|GetArrayItem` (`self.location`))) "AdjustIfPossibleButAlwaysSpawn" "OverrideRootScale" null null))
  (`Controller.Possess` (`GameplayStatics.GetPlayerControllerFromID` (`GameplayStatics.GetPlayerControllerID` NewPlayer)) _returnvalue))

(event `self.ReceiveTick`
  (params (DeltaSeconds :type "Float (single-precision)")))

(fn `UserConstructionScript`)