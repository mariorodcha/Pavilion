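; Smoke grenade actor (GranadaHumo) that releases a smoke effect when it explodes.
; Its Explota event spawns the P_ExitStair_Mist particle emitter at the actor's location and hides the static mesh.
; After a Duracion delay it destroys the emitter component and then itself.
; BeginPlay and construction only call their parent versions.
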(event `self.ReceiveBeginPlay`
  (`parent.ReceiveBeginPlay`))

(event `self.Explota`
  (bind _returnvalue (`GameplayStatics.SpawnEmitterAtLocation` "/Game/Efectos/P_ExitStair_Mist.P_ExitStair_Mist" (`self.K2_GetActorLocation`)))
  (`SceneComponent.SetVisibility` (`self.StaticMesh`) false false)
  (`KismetSystemLibrary.Delay` (`self.duracion`))
  (`ActorComponent.K2_DestroyComponent` _returnvalue)
  (`self.K2_DestroyActor`))

(fn `UserConstructionScript`
  (`parent.UserConstructionScript`))