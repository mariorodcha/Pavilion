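; Team base actor for a capture-the-flag mode that detects players entering its collision capsule.
; When an overlapping pawn's GamePlayPC has the same team ID and carries the flag, it clears the flag and calls FinRonda on GamePlayGM with that team, ending the round.
; Overlaps by players of another team only print a debug string with the base and player team IDs.
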(event `self.CollisionCapsule.OnComponentBeginOverlap`
  (params (OverlappedComponent :type "PrimitiveComponent Object Reference") (OtherActor :type "Actor Object Reference") (OtherComp :type "PrimitiveComponent Object Reference") (OtherBodyIndex :type Integer) (bFromSweep :type Boolean) (SweepResult :type "HitResult Structure (by ref)"))
  (bind _idequipo (`self.idEquipo`))
  (bind _aspawn (cast `Pawn` OtherActor))
  (bind _asgame_play_pc (cast `/Game/Blueprints/GamePlayMode/GamePlayPC` (`Pawn.GetController` _aspawn)))
  (bind _idequipo_2 (`/Game/Blueprints/GamePlayMode/GamePlayPC.idEquipo` _asgame_play_pc))
  (if (== _idequipo_2 _idequipo)
    (if (`/Game/Blueprints/GamePlayMode/GamePlayPC.tieneBandera?` _asgame_play_pc)
      (set `/Game/Blueprints/GamePlayMode/GamePlayPC.tieneBandera?` false _asgame_play_pc)
      (bind _asgame_play_gm (cast `/Game/Blueprints/GamePlayMode/GamePlayGM` (`GameplayStatics.GetGameMode`)))
      (`/Game/Blueprints/GamePlayMode/GamePlayGM.FinRonda` _asgame_play_gm (`self.idEquipo`)))
    (else
      (`KismetSystemLibrary.PrintString` (`KismetStringLibrary.BuildString_Int` (`KismetStringLibrary.BuildString_Int` "id base: " "" _idequipo) " id jugador:" _idequipo_2)))))

(fn `UserConstructionScript`)